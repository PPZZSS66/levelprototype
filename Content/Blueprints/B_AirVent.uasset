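; Air vent actor that pushes the player character upward while it is within a tall capsule-shaped area.
; Each Tick, a capsule overlap query at the Capsule component, filtered to the player's class, triggers a small additive upward LaunchCharacter on player 0 and a debug print.
; Separately, any actor beginning to overlap the vent plays Lift.
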(event `self.ReceiveBeginPlay`)

(event `self.ReceiveTick`
  (params (DeltaSeconds :type "Float (single-precision)"))
  (bind (_outactors _returnvalue) (`KismetSystemLibrary.CapsuleOverlapActors` (`SceneComponent.K2_GetComponentLocation` (`self.Capsule`)) 200.0 500.0 (`self.NewVar`) (`GameplayStatics.GetObjectClass` (`GameplayStatics.GetPlayerCharacter` 0))))
  (if _returnvalue
    (`Character.LaunchCharacter` (`GameplayStatics.GetPlayerCharacter` 0) (0.0 0.0 40.0) false false)
    (`KismetSystemLibrary.PrintString` "yes")))

(event `self.ReceiveActorBeginOverlap`
  (params (OtherActor :type "Actor Object Reference"))
  (`Timeline|Lift`))

(fn `UserConstructionScript`)