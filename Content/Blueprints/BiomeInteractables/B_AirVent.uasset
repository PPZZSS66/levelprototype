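; B_AirVent is an air vent interactable that pushes the third-person character upward.
; Entering the inner collision arms lifting, which only clears on leaving the larger collision.
; Entering the larger collision runs one guarded, delayed cycle that switches venting off, then back on.
; While both lifting and venting are true, Tick applies a small additive upward LaunchCharacter to player 0 and prints debug text.
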(event `self.ReceiveBeginPlay`)

(event `self.ReceiveTick`
  (params (DeltaSeconds :type "Float (single-precision)"))
  (if (`self.isLifting`)
    (if (`self.isVenting`)
      (`Character.LaunchCharacter` (`GameplayStatics.GetPlayerCharacter` 0) (0.0 0.0 40.0) false false)
      (`KismetSystemLibrary.PrintString` "yes"))))

(event `self.InitialCollision.OnComponentBeginOverlap`
  (params (OverlappedComponent :type "PrimitiveComponent Object Reference") (OtherActor :type "Actor Object Reference") (OtherComp :type "PrimitiveComponent Object Reference") (OtherBodyIndex :type Integer) (bFromSweep :type Boolean) (SweepResult :type "HitResult Structure (by ref)"))
  (cast `/Game/ThirdPerson/Blueprints/BP_ThirdPersonCharacter` OtherActor)
  (set `self.isLifting` true))

(event `self.InitialCollision.OnComponentEndOverlap`
  (params (OverlappedComponent :type "PrimitiveComponent Object Reference") (OtherActor :type "Actor Object Reference") (OtherComp :type "PrimitiveComponent Object Reference") (OtherBodyIndex :type Integer))
  (cast `/Game/ThirdPerson/Blueprints/BP_ThirdPersonCharacter` OtherActor))

(event `CycleVent`
  (bind _cycledelay (`self.cycleDelay`))
  (if (not (`self.isCycling`))
    (set `self.isCycling` true)
    (`KismetSystemLibrary.Delay` _cycledelay)
    (set `self.isVenting` false)
    (`KismetSystemLibrary.Delay` _cycledelay)
    (set `self.isVenting` true)
    (set `self.isCycling` false)))

(event `self.LargerCollision.OnComponentBeginOverlap`
  (params (OverlappedComponent :type "PrimitiveComponent Object Reference") (OtherActor :type "Actor Object Reference") (OtherComp :type "PrimitiveComponent Object Reference") (OtherBodyIndex :type Integer) (bFromSweep :type Boolean) (SweepResult :type "HitResult Structure (by ref)"))
  (cast `/Game/ThirdPerson/Blueprints/BP_ThirdPersonCharacter` OtherActor)
  (`self.CycleVent`))

(event `self.LargerCollision.OnComponentEndOverlap`
  (params (OverlappedComponent :type "PrimitiveComponent Object Reference") (OtherActor :type "Actor Object Reference") (OtherComp :type "PrimitiveComponent Object Reference") (OtherBodyIndex :type Integer))
  (cast `/Game/ThirdPerson/Blueprints/BP_ThirdPersonCharacter` OtherActor)
  (set `self.isLifting` false))

(fn `UserConstructionScript`)