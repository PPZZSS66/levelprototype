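; LinkingRuby is an interactable teleporter that moves the third-person player character to a linked PairedRuby.
; Overlap begin and end with BP_ThirdPersonCharacter set IsTouching and enable or disable this actor's player input.
; Pressing E while touching places the character at a small X offset from the paired ruby, then hands input from this ruby over to the paired one.
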(event `self.ReceiveTick`
  (params (DeltaSeconds :type "Float (single-precision)")))

(event `self.ReceiveBeginPlay`)

(event `self.ReceiveActorBeginOverlap`
  (params (OtherActor :type "Actor Object Reference"))
  ;[1 1 1] BeginOverlap
  (cast `/Game/ThirdPerson/Blueprints/BP_ThirdPersonCharacter` OtherActor)
  (set `self.isTouching` true)
  (`self.EnableInput` (`GameplayStatics.GetPlayerController` 0)))

(event `self.ReceiveActorEndOverlap`
  (params (OtherActor :type "Actor Object Reference"))
  ;[1 1 1] EndOverlap
  (cast `/Game/ThirdPerson/Blueprints/BP_ThirdPersonCharacter` OtherActor)
  (set `self.isTouching` false)
  (`self.DisableInput` (`GameplayStatics.GetPlayerController` 0)))

(event `Key|E`
  (params (Key :type "Key Structure"))
  (bind _returnvalue (`GameplayStatics.GetPlayerController` 0))
  ;[1 1 1] Teleport
  (:`Pressed`
    (if (`self.isTouching`)
      (cast `/Game/ThirdPerson/Blueprints/BP_ThirdPersonCharacter` (`GameplayStatics.GetPlayerCharacter` 0))
      (`self.K2_SetActorLocation` (`GameplayStatics.GetPlayerCharacter` 0) (+ (`SceneComponent.K2_GetComponentLocation` (`/Game/Blueprints/LinkingRuby.DefaultSceneRoot` (`self.pairedRuby`))) (50.0 0.0 0.0)) false false)
      (`self.DisableInput` _returnvalue)
      (`self.EnableInput` (`self.pairedRuby`) _returnvalue))))

(fn `UserConstructionScript`)