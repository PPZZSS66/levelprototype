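; Fairy NPC Blueprint that moves toward the player and shows dialogue when interacted with.
; When PawnSensing sees any pawn, it issues an AI MoveTo targeting the player character.
; Each Interact increments Talkindex, adds a Dialogue1 widget if UI is invalid, and sets its Talk text from the Dialog array at that index.
; Once the index exceeds the array length, Interact removes the widget.
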(event `self.PawnSensing.OnSeePawn`
  (params (Pawn :type "Pawn Object Reference"))
  (`|AIMoveTo` self (0.0 0.0 0.0) (`GameplayStatics.GetPlayerCharacter` 0)))

(event `self.Interact`
  (`/Engine/EditorBlueprintResources/StandardMacros.IncrementInt` (`self.talkindex`)
    (:`  `
      (if (<= (`self.talkindex`) (`KismetArrayLibrary.Array_Length` (`self.Dialog`)))
        (`self.UI`
          (:`then`
            _)
          (:`else`
            (`|CreateWidget` "/Game/UI/Dialogue1.Dialogue1_C" (`GameplayStatics.GetPlayerController` 0))
            (bind _output_get (set `self.UI` null))
            (`UserWidget.AddToViewport` (`self.UI`) 0)
            (`UserWidget.AddToViewport` _output_get 0)))
        (`TextBlock.SetText` (`/Game/UI/Dialogue.talk` (`self.UI`)) (`KismetTextLibrary.Conv_StringToText` (`|GetArrayItem` (`self.Dialog`) (`self.talkindex`))))
        (else
          (`Widget.RemoveFromParent` (`self.UI`)))))))

(fn `UserConstructionScript`)