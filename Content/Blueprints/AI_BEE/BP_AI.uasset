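; BP_AI is an AI pawn, apparently a bee, that wanders and chases the player.
; From BeginPlay, Walkaround moves to random reachable points nearby, repeating after a short delay only when a move succeeds.
; Pawn sensing sends it toward the player character on seeing any pawn.
; Overlapping the third-person character applies damage and prints a debug string, while its own TakeDamage function just returns zero.
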(event `self.PawnSensing.OnSeePawn`
  (params (Pawn :type "Pawn Object Reference"))
  (`|AIMoveTo` self (0.0 0.0 0.0) (`GameplayStatics.GetPlayerCharacter` 0)))

(event `self.ReceiveActorBeginOverlap`
  (params (OtherActor :type "Actor Object Reference"))
  (bind _asbp_third_person_character (cast `/Game/ThirdPerson/Blueprints/BP_ThirdPersonCharacter` OtherActor))
  (`GameplayStatics.ApplyDamage` _asbp_third_person_character 1.0)
  (`KismetSystemLibrary.PrintString` "NO"))

(event `Walkaround`
  (`|AIMoveTo` self (`NavigationSystemV1.K2_GetRandomReachablePointInRadius` (`self.K2_GetActorLocation`) 2000.0 null null) null 500.0
    (:`OnSuccess`
      (`KismetSystemLibrary.Delay` 2.0)
      (`self.Walkaround`))))

(event `self.ReceiveBeginPlay`
  (`self.Walkaround`))

(fn `TakeDamage`
  (params (DamageAmount :type "Float (double-precision)"))
  (returns (DamageDealt :type "Float (double-precision)"))
  (return 0.0))

(fn `UserConstructionScript`)