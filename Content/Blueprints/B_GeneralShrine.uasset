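; B_GeneralShrine is a save-point shrine that saves the game when the player character overlaps it.
; On overlap it calls SaveTheGame on BP_ThirdPersonCharacter, waits briefly, then brightens its point light and reveals a sphere if the save slot exists.
; Any other overlapping actor prints a failure message.
; Level-loading logic that reads the saved level name remains in the graph but is unconnected.
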(event `self.ReceiveActorBeginOverlap`
  (params (OtherActor :type "Actor Object Reference"))
  (bind _asbp_third_person_character (cast `/Game/ThirdPerson/Blueprints/BP_ThirdPersonCharacter` OtherActor)
    (:`then`
      (`/Game/ThirdPerson/Blueprints/BP_ThirdPersonCharacter.SaveTheGame` _asbp_third_person_character)
      (`KismetSystemLibrary.PrintString` "Saving the Game...")
      (`KismetSystemLibrary.Delay` 0.2)
      (bind _returnvalue (`GameplayStatics.DoesSaveGameExist` (`/Game/ThirdPerson/Blueprints/BP_ThirdPersonCharacter.Slot Name` _asbp_third_person_character)))
      (if _returnvalue
        (`LightComponent.SetIntensity` (`self.PointLight`) 150.0)
        (`SceneComponent.SetVisibility` (`self.Sphere`) true false)))
    (:`CastFailed`
      (`KismetSystemLibrary.PrintString` "Game save failed..."))))

(fn `UserConstructionScript`)